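; BP_WarpZone is a two-way warp actor that teleports the player between two trigger boxes.
; When a ThirdPersonCharacter overlaps either WarpBox, player character 0 is teleported to the arrow paired with the other box, with its rotation reset to zero.
; Each warp spawns a scaled-up P_Warp particle effect at the destination and plays a shared 2D teleport sound.
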(event OnComponentBeginOverlap(WarpBox_01)
  (params (OverlappedComponent :type Primitive%20Component%20Object%20Reference) (OtherActor :type Actor%20Object%20Reference) (OtherComp :type Primitive%20Component%20Object%20Reference) (OtherBodyIndex :type Integer) (bFromSweep :type Boolean) (SweepResult :type Hit%20Result%20Structure%20%28by%20ref%29))
  (bind _arrow_02 (Variables|Default|GetArrow_02))
  (bind _returnvalue (Transformation|GetWorldLocation _arrow_02))
  (Utilities|Casting|CastToThirdPersonCharacter OtherActor)
  (Transformation|Teleport (Game|GetPlayerCharacter 0) _returnvalue "0, 0, 0")
  (Effects|SpawnEmitteratLocation "/Game/InfinityBladeEffects/Effects/FX_Ability/Defense/P_Warp.P_Warp" _returnvalue "0, 0, 0" "2.000000,2.000000,2.000000")
  (Audio|PlaySound2D "/Engine/VREditor/Sounds/UI/Teleport_Committed.Teleport_Committed" 2.0 1.0 0.0 0 0))

(event OnComponentBeginOverlap(WarpBox_02)
  (params (OverlappedComponent :type Primitive%20Component%20Object%20Reference) (OtherActor :type Actor%20Object%20Reference) (OtherComp :type Primitive%20Component%20Object%20Reference) (OtherBodyIndex :type Integer) (bFromSweep :type Boolean) (SweepResult :type Hit%20Result%20Structure%20%28by%20ref%29))
  (bind _arrow_01 (Variables|Default|GetArrow_01))
  (bind _returnvalue (Transformation|GetWorldLocation _arrow_01))
  (Utilities|Casting|CastToThirdPersonCharacter OtherActor)
  (Transformation|Teleport (Game|GetPlayerCharacter 0) _returnvalue "0, 0, 0")
  (Effects|SpawnEmitteratLocation "/Game/InfinityBladeEffects/Effects/FX_Ability/Defense/P_Warp.P_Warp" _returnvalue "0, 0, 0" "2.000000,2.000000,2.000000")
  (Audio|PlaySound2D "/Engine/VREditor/Sounds/UI/Teleport_Committed.Teleport_Committed" 2.0 1.0 0.0 0 0))

(fn ConstructionScript)