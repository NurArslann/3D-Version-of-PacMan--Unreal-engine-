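; BP_PowerUp_Speed is a speed power-up pickup that boosts a ThirdPersonCharacter when it overlaps the pickup's sphere.
; On overlap it calls the character's SPEEDBOOST, plays a sound, activates SFXEaten, and destroys the mesh, sphere and glow components.
; The actor destroys itself after a short delay.
; A separate SpawnFX function, not called within this Blueprint, plays an enlarged particle burst and spawn sound at the sphere's location.
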(event OnComponentBeginOverlap(Sphere)
  (params (OverlappedComponent :type Primitive%20Component%20Object%20Reference) (OtherActor :type Actor%20Object%20Reference) (OtherComp :type Primitive%20Component%20Object%20Reference) (OtherBodyIndex :type Integer) (bFromSweep :type Boolean) (SweepResult :type Hit%20Result%20Structure%20%28by%20ref%29))
  ;[1 1 1] Power Up Eaten
  (bind _asthird_person_character (Utilities|Casting|CastToThirdPersonCharacter OtherActor))
  (Default|SPEEDBOOST _asthird_person_character)
  (Audio|PlaySound2D "/Game/Audio/SFX_EatSpecial_Cue.SFX_EatSpecial_Cue" 1.0 1.0 0.0 0 0)
  (Components|Activation|Activate (Variables|Default|GetSFX_Eaten) false)
  (Components|DestroyComponent (Variables|Default|GetSM_Booster))
  (Utilities|FlowControl|Delay 5.0)
  (Actor|DestroyActor))

(fn ConstructionScript)

(fn SpawnFX
  (bind _returnvalue (Effects|SpawnEmitteratLocation "/Game/InfinityBladeEffects/Effects/FX_Mobile/Misc/P_levelUp.P_levelUp" (Transformation|GetWorldLocation (Variables|Default|GetSphere))))
  (Transformation|SetWorldScale3D _returnvalue "3.000000,3.000000,3.000000")
  (Audio|PlaySound2D "/Game/Audio/SFX_FruitSpawn_Cue.SFX_FruitSpawn_Cue" 1.0 1.0 0.0 0 0))