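; Parent Blueprint for Pac-Man-style ghost enemies that wander or hunt the player.
; A start timer repeats until the player can gobble, then opens a Tick-fed gate driving AI moves to random TargetPoints or the player.
; Power pellets play a timeline that steps through two vulnerable looks before restoring normal state.
; On overlap, a vulnerable ghost respawns at home with effects; otherwise it signals a player kill and resets all enemies.
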(event OnComponentBeginOverlap(Player_Collision)
  (params (OverlappedComponent :type Primitive%20Component%20Object%20Reference) (OtherActor :type Actor%20Object%20Reference) (OtherComp :type Primitive%20Component%20Object%20Reference) (OtherBodyIndex :type Integer) (bFromSweep :type Boolean) (SweepResult :type Hit%20Result%20Structure%20%28by%20ref%29))
  ;[1 1 1] Enemy Toched Player
  (bind _asthird_person_character (Utilities|Casting|CastToThirdPersonCharacter OtherActor))
  (Utilities|IsValid _asthird_person_character
    (:Is%20Valid
      (if (Variables|Default|GetbIdVulnerable?)
        (CallFunction|CloseEnemyNavGate)
        (CallFunction|EnemyEatenFX)
        ;[1 1 1] enemy eaten respawn enemy back home
        (Collision|SetCollisionResponsetoChannel (Variables|Default|GetPlayer_Collision) "ECC_Pawn" "ECR_Ignore")
        (Variables|Default|SetbIdVulnerable? true)
        (CallFunction|EnemyStateRegular)
        (Transformation|SetActorLocation (Variables|ChildParemeters|GetEnemyRespwanLocation) false false)
        (Utilities|FlowControl|Delay 2.0)
        (Effects|SpawnEmitteratLocation "/Game/InfinityBladeEffects/Effects/FX_Monsters/FX_Monster_Deaths/P_Monster_Death_Large.P_Monster_Death_Large" (Variables|ChildParemeters|GetEnemyRespwanLocation)) ; respawn
        (Collision|SetCollisionResponsetoChannel (Variables|Default|GetPlayer_Collision) "ECC_Pawn" "ECR_Ignore")
        (Utilities|FlowControl|Delay 1.0)
        (Rendering|SetActorHiddenInGame false)
        (else
          (Default|CallKilledPlayer)
          (CallFunction|CloseEnemyNavGate (Variables|References|GetEnemies))
          ;[1 1 1] send all enemies home
          (Utilities|FlowControl|Delay 2.5)
          (CallFunction|ResetEnemiestoHouse (Variables|References|GetEnemies)))))))

(event Custom|Set%20Enemy%20Start%20Time
  ;[1 1 1] Start Enmy Nav
  (Utilities|Time|SetTimerbyEvent (delegate Custom|Start%20Nav) (Variables|ChildParemeters|GetEnemyStartTime)))

(event Custom|KilledPlayer_Event)

(event Custom|Power%20Pellet%20Eatan
  ;[1 1 1] Vulnerability Sequence
  (Variables|Default|SetbIdVulnerable? true)
  (Default|CallVulnerable) ; Calls event in game mode BP_Gmaes music
  (Timeline|Vulnerability%20Sequence PlayFromStart
    (:Finished
      (CallFunction|EnemyStateRegular)
      (Variables|Default|SetbIdVulnerable? false)
      (if (Variables|ChildParemeters|GetbIsWanderGhost?)
        (Variables|ChildParemeters|SetEnemyNavType "NewEnumerator1")
        (else
          (Variables|ChildParemeters|SetEnemyNavType "NewEnumerator0")))
      (Default|CallNotVulnerable))
    (:Start%20Phaze%20#1
      (CallFunction|EnemyStateVulnarable01))
    (:Start%20Phaze%20#2
      (if (Variables|Default|GetbIdVulnerable?) ; is it still vunerable?
        (CallFunction|EnemyStateVulnarable02)))))

(event Custom|Reset%20Enemies%20to%20house
  (CallFunction|EnemySpawnOutFX)
  ;[1 1 1] enemy eaten respawn enemy back home
  (Transformation|SetActorLocation (Variables|ChildParemeters|GetEnemyRespwanLocation) false false)
  (Utilities|FlowControl|Delay 2.0)
  (Effects|SpawnEmitteratLocation "/Game/InfinityBladeEffects/Effects/FX_Monsters/FX_Monster_Deaths/P_Monster_Death_Large.P_Monster_Death_Large" (Variables|ChildParemeters|GetEnemyRespwanLocation)) ; respawn
  (Collision|SetCollisionResponsetoChannel (Variables|Default|GetPlayer_Collision) "ECC_Pawn" "ECR_Ignore")
  (Utilities|FlowControl|Delay 1.0)
  (Rendering|SetActorHiddenInGame false))

(event Custom|Start%20Nav
  ;[1 1 1] Start Enmy Nav
  (if (Variables|/Game/Blueprints/Character/ThirdPersonCharacter.ThirdPersonCharacter_C|GetbShouldPlayerGobble? (Variables|References|GetPlayer))
    (Components|Activation|Activate (Variables|Character|GetCharacterMovement) false)
    (Variables|Navigation|SetbAssignedTargetPoint false)
    (Utilities|FlowControl|Gate true) ; enters at Open
    (else
      (Utilities|Time|SetTimerbyEvent (delegate Custom|Start%20Nav) (Variables|ChildParemeters|GetEnemyStartTime)))))

(event Custom|Pick%20New%20Nav%20Point
  ;[1 1 1] Pick New Nav Point
  (Utilities|FlowControl|Delay 0.1)
  (Variables|Navigation|SetbAssignedTargetPoint false)
  (Utilities|FlowControl|Gate true) ; enters at Open
)

(event Custom|Close%20Enemy%20Nav%20Gate
  ;[1 1 1] Stop Enemy Nav
  (Components|Activation|Deactivate (Variables|Character|GetCharacterMovement))
  (Utilities|FlowControl|Gate true) ; enters at Close
)

(event EventBeginPlay
  (Utilities|FlowControl|Sequence
    (:then_0
      ;[1 1 1] refence to all enemies
      (bind _outactors (Actor|GetAllActorsOfClass "BP_Enemy_Parent_C"))
      (Variables|References|SetEnemies _outactors)
      (bind _asthird_person_character (Utilities|Casting|CastToThirdPersonCharacter (Game|GetPlayerCharacter 0)))
      (Variables|References|SetPlayer _asthird_person_character)
      ;[1 1 1] reference to target points
      (bind _outactors_2 (Actor|GetAllActorsOfClass "/Script/Engine.TargetPoint"))
      (Variables|References|Settarget%20Points _outactors_2))
    (:then_1
      ;[1 1 1] Open Gate for Enemy Navigation
      (CallFunction|SetEnemyStartTime))))

(event EventTick
  (params (DeltaSeconds :type Float%20%28single-precision%29))
  (Development|PrintString (Utilities|GetDisplayName (Variables|Navigation|GetEnemySelectedTarget)))
  (Utilities|FlowControl|Gate true
    (:Exit
      (switch Utilities|FlowControl|Switch|SwitchonEnemyNavType (Variables|ChildParemeters|GetEnemyNavType)
        (:NewEnumerator0
          (if (Variables|Navigation|GetbAssignedTargetPoint)
            ;[1 1 1] Enemy Got  to Target Point? -Then Pick New Location
            (if (<= (Transformation|GetDistanceTo self (Variables|Navigation|GetEnemySelectedTarget)) (Variables|ChildParemeters|GetEnemyTargetAcceptenceRadius))
              (CallFunction|PickNewNavPoint))
            (else
              ;[1 1 1] wander Enemy Nav
              (CallFunction|NavigationWander))))
        (:NewEnumerator1
          ;[1 1 1] Hunter Enemy Nav
          (CallFunction|NavigationHunter))))))

(fn ConstructionScript)

(fn EnemyStateRegular
  (Rendering|SetVisibility (Variables|Default|GetEnemy_Vulnerable) false false)
  (Rendering|SetVisibility (Variables|Default|GetEnemy_Down) true false))

(fn EnemyStateVulnarable01
  (Rendering|SetVisibility (Variables|Default|GetEnemy_Vulnerable_02) false false)
  (Rendering|SetVisibility (Variables|Default|GetEnemy_Vulnerable) true false))

(fn EnemyStateVulnarable02
  (Rendering|SetVisibility (Variables|Default|GetEnemy_Vulnerable) false false)
  (Rendering|SetVisibility (Variables|Default|GetEnemy_Vulnerable_02) true false))

(fn EnemyEatenFX
  (Effects|SpawnEmitteratLocation "/Game/StarterContent/Particles/P_Death.P_Death" (Transformation|GetWorldLocation (Variables|Collision|GetCapsuleComponent)) "0, 0, 0" "3.000000,3.000000,3.000000")
  (Audio|SpawnSound2D "/Game/StarterContent/Audio/Explosion_Cue.Explosion_Cue" 1.0 1.0 0.0 0)
  (Rendering|SetActorHiddenInGame true))

(fn EnemySpawnOutFX
  (Effects|SpawnEmitteratLocation "/Game/InfinityBladeEffects/Effects/FX_Skill_Leap/P_SpawnOutEnemy.P_SpawnOutEnemy" (Transformation|GetWorldLocation (Variables|Collision|GetCapsuleComponent)))
  (Rendering|SetActorHiddenInGame true))

(fn NavigationWander
  (bind _target_points (Variables|References|Gettarget%20Points))
  (bind _output_get (Variables|Navigation|SetEnemySelectedTarget (Utilities|Array|Get(acopy) _target_points (Math|Random|RandomInteger (Utilities|Array|Length _target_points)))))
  (AI|Navigation|MovetoLocation (AI|GetAIController (Pawn|GetController)) (Transformation|GetActorLocation _output_get) -1.0 true true false true 0)
  (Variables|Navigation|SetbAssignedTargetPoint true))

(fn NavigationHunter
  (AI|Navigation|MovetoLocation (AI|GetAIController (Pawn|GetController)) (Transformation|GetWorldLocation (Variables|/Script/Engine.Character|GetCapsuleComponent (Variables|References|GetPlayer))) -1.0 true true false true 0))