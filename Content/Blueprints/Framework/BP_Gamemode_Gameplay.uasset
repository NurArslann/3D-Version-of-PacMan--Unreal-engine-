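; Gameplay game mode for a Pac-Man-style level that tracks pellets, intro camera, bonus spawning and music.
; BeginPlay counts regular and power pellets, blends to a gameplay camera with input disabled, and schedules one random fruit or speed power-up.
; Each ATE event decrements the count; at zero it stops the player and fires LevelCompleted.
; Enemy killed-player and vulnerability dispatchers, plus LevelCompleted, control the gameplay and vulnerable music tracks.
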(event Custom|ATE
  (bind _playerref (Variables|Default|GetPlayerRef))
  ;[1 1 1] Level Complition Check
  (bind _result (Math|Integer|DecrementInt (Variables|LevelStatus|GetTotalPellets))
    (:%20%20
      (bind _output_get (Variables|LevelStatus|SetTotalPellets _result))
      (if (<= _output_get 0)
        (Variables|Spawning|SetbGoodieSpawnOK false)
        (Utilities|FlowControl|Sequence
          (:then_0
            ;[1 1 1] Stop P;layer Nav
            (Input|DisableInput (Game|GetPlayerCharacter 0) (Game|GetPlayerController 0))
            (Variables|/Script/Engine.CharacterMovementComponent|SetMaxWalkSpeed (Variables|/Script/Engine.Character|GetCharacterMovement _playerref) 0.0)
            (Variables|/Game/Blueprints/Character/ThirdPersonCharacter.ThirdPersonCharacter_C|SetbShouldPlayerGobble? _playerref false))
          (:then_1
            (Development|PrintString "End of Levell" true true "(R=0.000000,G=0.660000,B=1.000000,A=1.000000)" 1e+01))
          (:then_2
            (CallFunction|LevelCompletedEvent)))))))

(event Custom|KilledPlayer_Event_0
  (bind _music_gameplay (Variables|Default|GetMusic_GamePlay))
  ;[1 1 1] Music Stop when player stop
  (Utilities|FlowControl|Sequence
    (:then_0
      (Audio|Components|Audio|Stop _music_gameplay))
    (:then_1
      (Utilities|FlowControl|Delay 7.0)
      (Audio|Components|Audio|FadeIn _music_gameplay 0.5 1.0 7.0 "Linear" :!class /Script/Engine.AudioComponent))))

(event Custom|Vulnerable_Event_0
  (bind _music_vulnerable (Variables|Default|GetMusic_Vulnerable))
  ;[1 1 1] Enemies Vulnerble or not?
  (Class|AudioComponent|SetPaused (Variables|Default|GetMusic_GamePlay) true)
  (if (not (Audio|Components|Audio|IsPlaying _music_vulnerable))
    (Audio|Components|Audio|Play _music_vulnerable 0.0)))

(event Custom|NotVulnerable_Event_0
  ;[1 1 1] Enemies Vulnerble or not?
  (Class|AudioComponent|SetPaused (Variables|Default|GetMusic_GamePlay) false)
  (Audio|Components|Audio|Stop (Variables|Default|GetMusic_Vulnerable)))

(event Custom|LevelCompleted_Event
  ;[1 1 1] Level Complete stop music
  (Utilities|FlowControl|Delay 0.1)
  (Audio|Components|Audio|Stop (Variables|Default|GetMusic_GamePlay)))

(event EventBeginPlay
  (bind _returnvalue (Game|GetPlayerCharacter 0))
  (bind _goodie__spawn_01 (Variables|Goodies|GetGoodie%20%20Spawn_01))
  (bind _goodie__spawn_02 (Variables|Goodies|GetGoodie%20%20Spawn_02))
  (bind _array (Utilities|Array|MakeArray _goodie__spawn_01 _goodie__spawn_02))
  (Utilities|FlowControl|Sequence
    (:then_0
      (bind _asthird_person_character (Utilities|Casting|CastToThirdPersonCharacter (Game|GetPlayerCharacter 0)))
      (Variables|Default|SetPlayerRef _asthird_person_character)
      ;[1 1 1] Reference to all enemies
      (bind _outactors (Actor|GetAllActorsOfClass "/Game/Blueprints/Character/BP_Enemy_Parent.BP_Enemy_Parent_C"))
      (Variables|References|SetEemies _outactors))
    (:then_2
      (bind _outactors_2 (Actor|GetAllActorsOfClass "/Game/Blueprints/Pickups/BP_Pellet.BP_Pellet_C"))
      (bind _output_get (Variables|LevelStatus|SetTotalRegularPellets (Utilities|Array|Length _outactors_2)))
      (bind _output_get_2 (Variables|LevelStatus|SetTotalPellets (+ _output_get (stale _output_get_3)) :!label _label))
      (Development|PrintString (Utilities|String|ToString(Integer) _output_get_2) true true "(R=1.000000,G=0.126379,B=0.903951,A=1.000000)" 5.0))
    (:then_3
      (bind _outactors_3 (Actor|GetAllActorsOfClass "/Game/Blueprints/Pickups/BP_PowerPellet.BP_PowerPellet_C"))
      (bind _output_get_3 (Variables|LevelStatus|SetTotalPowerPellets (Utilities|Array|Length _outactors_3)))
      (goto _label))
    (:then_4
      (Input|DisableInput (Game|GetPlayerCharacter 0) (Game|GetPlayerController 0))
      (bind _returnvalue_2 (Game|SpawnActorfromClass "/Script/Engine.CameraActor" (Math|Transform|MakeTransform (Variables|Camera|GetCamGamePlay_Loc) (Variables|Camera|GetCamGamePlay_Rot) "1,1,1") "Undefined" 0 0))
      (Game|Player|SetViewTargetwithBlend (Game|GetPlayerController 0) _returnvalue_2 6.8 "VTBlend_Linear" 0.0 false)
      (Utilities|FlowControl|Delay 7.0)
      (Input|EnableInput _returnvalue (Game|GetPlayerController 0))
      (bind _asthird_person_character_2 (Utilities|Casting|CastToThirdPersonCharacter _returnvalue))
      (Variables|/Game/Blueprints/Character/ThirdPersonCharacter.ThirdPersonCharacter_C|SetbAllowedToMove? _asthird_person_character_2 true))
    (:then_5
      ;[1 1 1] Fruit/Power Up Spawn
      (Utilities|FlowControl|Delay (Math|Random|RandomFloatinRange 25.0 5e+01))
      (if (Variables|Spawning|GetbGoodieSpawnOK)
        (bind _output_get_4 (Variables|Goodies|SetGoodieSpawnLocales _array))
        (switch int (Math|Random|RandomIntegerinRange 0 2)
          (:0
            (Game|SpawnActorfromClass "/Game/Blueprints/Pickups/BP_Food_Cherry.BP_Food_Cherry_C" (Math|Conversions|ToTransform(Vector) (Utilities|Array|Get(acopy) _output_get_4 (Math|Random|RandomIntegerinRange 0 (- (Utilities|Array|Length _array) 1)))) "Undefined" 0 0))
          (:1
            (Game|SpawnActorfromClass "/Game/Blueprints/Pickups/BP_Food_Orange.BP_Food_Orange_C" (Math|Conversions|ToTransform(Vector) (Utilities|Array|Get(acopy) _output_get_4 (Math|Random|RandomIntegerinRange 0 (- (Utilities|Array|Length _array) 1)))) "Undefined" 0 0))
          (:2
            (Game|SpawnActorfromClass "/Game/Blueprints/Pickups/BP_PowerUp_Speed.BP_PowerUp_Speed_C" (Math|Conversions|ToTransform(Vector) (Utilities|Array|Get(acopy) _output_get_4 (Math|Random|RandomIntegerinRange 0 (- (Utilities|Array|Length _array) 1)))) "Undefined" 0 0)))))
    (:then_6
      (Utilities|FlowControl|Sequence
        (:then_0
          ;[1 1 1] Music Stop when player stop
          (EventDispatchers|AssignKilledPlayer (Variables|References|GetEemies) (delegate Custom|KilledPlayer_Event_0)))
        (:then_1
          ;[1 1 1] Enemies Vulnerble or not?
          (EventDispatchers|AssignVulnerable (Variables|References|GetEemies) (delegate Custom|Vulnerable_Event_0)))
        (:then_2
          (EventDispatchers|AssignNotVulnerable (Variables|References|GetEemies) (delegate Custom|NotVulnerable_Event_0)))
        (:then_3
          ;[1 1 1] Level Complete stop music
          (EventDispatchers|BindEventtoLevelCompleted (delegate Custom|LevelCompleted_Event)))))))

(fn ConstructionScript)